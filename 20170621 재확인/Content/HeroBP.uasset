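; Player hero character with camera-relative movement, a punch state and a mouse-placed click marker.
; BeginPlay spawns the MousePointBP marker and shows the cursor; left click moves it to the cursor hit and holds IsPunching until released.
; Tick lerps control rotation toward Target, while Turn axes share a rotation routine gated on near-zero input.
; The construction script snaps left and right sphere components to the mesh's hand sockets.
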(event `self.ReceiveBeginPlay`
  (bind _returnvalue (`|SpawnActorFromClass` "/Game/UI/MousePointBP.MousePointBP_C" (`KismetMathLibrary.Conv_VectorToTransform` (`self.K2_GetActorLocation`)) "Undefined" "OverrideRootScale"))
  (set `self.MouseClickPoint` _returnvalue)
  (set `PlayerController.bShowMouseCursor` true (`GameplayStatics.GetPlayerController` 0)))

(event `InputAxis|MoveForwardRear`
  (params (AxisValue :type "Float (single-precision)"))
  (`self.AddMovementInput` (`KismetMathLibrary.GetForwardVector` (`KismetMathLibrary.MakeRotator` 0.0 0.0 (.yaw (`self.GetControlRotation`)))) AxisValue))

(event `self.ReceiveTick`
  (params (DeltaSeconds :type "Float (single-precision)"))
  (`self.Rotate`))

(event `InputAction|LeftMouseClicked`
  (params (Key :type "Key Structure" :default "AnyKey"))
  (:`Pressed`
    (`self.K2_SetActorLocation` (`self.MouseClickPoint`) (`.Location` (`GameplayStatics.BreakHitResult` (`PlayerController.GetHitResultUnderCursorByChannel` (`GameplayStatics.GetPlayerController` 0) "TraceTypeQuery1" true))) false false)))

(event `InputAxis|MoveLeftRight`
  (params (AxisValue :type "Float (single-precision)"))
  (`self.AddMovementInput` (`KismetMathLibrary.GetRightVector` (`KismetMathLibrary.MakeRotator` 0.0 0.0 (.yaw (`self.GetControlRotation`)))) AxisValue))

(event `InputAction|LeftMouseClicked`
  (params (Key :type "Key Structure" :default "AnyKey"))
  (:`Pressed`
    (set `self.IsPunching` true))
  (:`Released`
    (set `self.IsPunching` false)))

(event `InputAxis|TurnForward`
  (params (AxisValue :type "Float (single-precision)"))
  (bind _returnvalue (`KismetMathLibrary.MakeVector` AxisValue (stale `InputAxis|Turn` AxisValue)))
  (if (`KismetMathLibrary.NearlyEqual_FloatFloat` (`KismetMathLibrary.VSizeSquared` _returnvalue)) :!label _label
    (`self.K2_SetActorRotation` (`KismetMathLibrary.Conv_VectorToRotator` _returnvalue))))

(event `InputAxis|Turn`
  (params (AxisValue :type "Float (single-precision)"))
  (goto _label))

(fn `Rotate`
  (`Controller.SetControlRotation` (`self.GetController`) (`KismetMathLibrary.RLerp` (`self.GetControlRotation`) (`self.Target`))))

(fn `UserConstructionScript`
  (bind _mesh (`self.Mesh`))
  (`SceneComponent.K2_AttachToComponent` (`self.RightHandSphere`) _mesh "hand_r" "SnapToTarget" "SnapToTarget" "KeepWorld" true)
  (`SceneComponent.K2_AttachToComponent` (`self.LeftHandSphere`) _mesh "hand_l" "SnapToTarget" "SnapToTarget" "KeepWorld" true))